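; Cauldron actor for a potion-brewing puzzle that needs a blue potion, red herbs and a green mushroom.
; Overlap checks actor tags, sets that ingredient's flag or GameOver for a wrong color, then calls DestroyActor on the pot itself.
; Tick prints a Polish success or Baba Jaga failure message from those flags.
; Tick also shows GhostSmoke only while the player character has a GhostCamera-tagged camera component.
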(event `self.ReceiveBeginPlay`
  (set `self.CorrectPotion ` false)
  (set `self.CorrectMushroom` false)
  (set `self.CorrectHerbs` false)
  (set `self.GameOver` false))

(event `self.ReceiveTick`
  (params (DeltaSeconds :type "Float (single-precision)"))
  (bind _ghostsmoke (`self.GhostSmoke`))
  (if (`KismetArrayLibrary.Array_IsNotEmpty` (`self.GetComponentsByTag` (`GameplayStatics.GetPlayerCharacter` 0) "/Script/Engine.CameraComponent" "GhostCamera"))
    (`SceneComponent.SetVisibility` _ghostsmoke true false)
    (else
      (`SceneComponent.SetVisibility` _ghostsmoke false false)))
  (if (and (`self.CorrectPotion `) (`self.CorrectMushroom`) (`self.CorrectHerbs`))
    (`KismetSystemLibrary.PrintString` "ZAJEBISTA MIKSTURA MORDECZKO")
    (elif (`self.GameOver`)
      (`KismetSystemLibrary.PrintString` "BABA JAGA CIE ZJE JELOPIE"))))

(event `self.ReceiveActorBeginOverlap`
  (params (OtherActor :type "Actor Object Reference"))
  (if (`self.ActorHasTag` OtherActor "Potion")
    (if (`self.ActorHasTag` OtherActor "Blue")
      (set `self.CorrectPotion ` true)
      (else
        (set `self.GameOver` true :!label _label)))
    (`self.K2_DestroyActor` :!label _label_2)
    (elif (`self.ActorHasTag` OtherActor "Herbs")
      (if (`self.ActorHasTag` OtherActor "Red")
        (set `self.CorrectHerbs` true)
        (goto _label_2)
        (else
          (goto _label)))
      (elif (`self.ActorHasTag` OtherActor "Mushroom")
        (if (`self.ActorHasTag` OtherActor "Green")
          (set `self.CorrectMushroom` true)
          (goto _label_2)
          (else
            (goto _label)))))))

(fn `UserConstructionScript`)