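; Playable ghost character that floats up and down and interacts with the world through a first-person camera.
; Each Tick runs a debug-drawn camera line trace, whose hit feeds the grab and drag inputs.
; Grab toggles particles on Candle-tagged actors, or toggles Fire particles on SpiderNet actors and destroys them after a delay.
; Drag grabs the hit component with a physics handle; logic for moving Movable-tagged actors is unconnected.
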(event `EnhancedInput|/Game/FirstPersonContentPack/FirstPerson/Input/Actions/IA_Float`
  (params (ActionValue :type Boolean) (ElapsedSeconds :type "Float (double-precision)") (TriggeredSeconds :type "Float (double-precision)") (InputAction :type "InputAction Object Reference" :default "/Game/FirstPersonContentPack/FirstPerson/Input/Actions/IA_Float.IA_Float"))
  (:`Ongoing`
    (`self.K2_AddActorWorldOffset` (0.0 0.0 15.0))))

(event `EnhancedInput|/Game/FirstPersonContentPack/FirstPerson/Input/Actions/IA_Crouch`
  (params (ActionValue :type Boolean) (ElapsedSeconds :type "Float (double-precision)") (TriggeredSeconds :type "Float (double-precision)") (InputAction :type "InputAction Object Reference" :default "/Game/FirstPersonContentPack/FirstPerson/Input/Actions/IA_Crouch.IA_Crouch"))
  (:`Ongoing`
    (`self.K2_AddActorWorldOffset` (0.0 0.0 -10.0))))

(event `EnhancedInput|/Game/FirstPersonContentPack/FirstPerson/Input/Actions/IA_Grab`
  (params (ActionValue :type Boolean) (ElapsedSeconds :type "Float (double-precision)") (TriggeredSeconds :type "Float (double-precision)") (InputAction :type "InputAction Object Reference" :default "/Game/FirstPersonContentPack/FirstPerson/Input/Actions/IA_Grab.IA_Grab"))
  (:`Started`
    (`KismetSystemLibrary.DrawDebugSphere` (stale `self.ReceiveTick` _impactpoint) 50.0)
    (if (`self.ActorHasTag` (stale `self.ReceiveTick` _hitactor) "Candle")
      (`SceneComponent.ToggleVisibility` (`self.GetComponentByClass` (stale `self.ReceiveTick` _hitactor) "/Script/Engine.ParticleSystemComponent") false)
      (elif (`self.ActorHasTag` (stale `self.ReceiveTick` _hitactor) "SpiderNet")
        (bind _output_get (set `self.SavedActor` (stale `self.ReceiveTick` _hitactor)))
        (for _array_element (`self.GetComponentsByTag` (stale `self.ReceiveTick` _hitactor) "/Script/Engine.ParticleSystemComponent" "Fire")
          (`SceneComponent.ToggleVisibility` _array_element false)
          (`KismetSystemLibrary.Delay` 3.0)
          (`self.K2_DestroyActor` _output_get))))))

(event `self.ReceiveTick`
  (params (DeltaSeconds :type "Float (single-precision)"))
  (bind (_impactpoint _hitactor _hitcomponent) (`self.LineTraceGetHit`)))

(event `EnhancedInput|/Game/FirstPersonContentPack/FirstPerson/Input/Actions/IA_Drag`
  (params (ActionValue :type Boolean) (ElapsedSeconds :type "Float (double-precision)") (TriggeredSeconds :type "Float (double-precision)") (InputAction :type "InputAction Object Reference" :default "/Game/FirstPersonContentPack/FirstPerson/Input/Actions/IA_Drag.IA_Drag"))
  (:`Started`
    (`PhysicsHandleComponent.GrabComponentAtLocation` (`self.PhysicsHandle`) (stale `self.ReceiveTick` _hitcomponent) "None" (stale `self.ReceiveTick` _impactpoint))))

(fn `LineTraceGetHit`
  (returns (ImpactPoint :type "Vector Structure") (HitActor :type "Actor Object Reference") (HitComponent :type "PrimitiveComponent Object Reference"))
  (bind _firstpersoncamera (`self.FirstPersonCamera`))
  (bind _returnvalue (`SceneComponent.K2_GetComponentLocation` _firstpersoncamera))
  (bind _outhit (`KismetSystemLibrary.LineTraceSingle` :`Start` _returnvalue :`End` (+ _returnvalue (* (`KismetMathLibrary.GetForwardVector` (`SceneComponent.K2_GetComponentRotation` _firstpersoncamera)) 500.0)) :`TraceChannel` "TraceTypeQuery1" :`DrawDebugType` "ForOneFrame"))
  (bind (_bblockinghit _binitialoverlap _time _distance _location _impactpoint _normal _impactnormal _physmat _hitactor _hitcomponent) (`GameplayStatics.BreakHitResult` _outhit))
  (if _bblockinghit
    (return _impactpoint _hitactor _hitcomponent)))

(fn `UserConstructionScript`
  (`parent.UserConstructionScript`))