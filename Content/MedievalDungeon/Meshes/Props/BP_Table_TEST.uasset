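; Test table prop with a BPCandle component that is visible only while the player character has a camera component tagged GhostCamera.
; The candle starts hidden, and Tick calls ChangeVisibilityGhostCamera to re-check for that tagged component and set visibility every frame.
; Any overlapping actor tagged Candle is destroyed, independently of the candle's visibility.
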(event `self.ReceiveBeginPlay`
  (`SceneComponent.SetVisibility` (`self.BP_Candle`) false false))

(event `self.ReceiveTick`
  (params (DeltaSeconds :type "Float (single-precision)"))
  (`self.ChangeVisibilityGhostCamera` (`self.BP_Candle`)))

(event `self.ReceiveActorBeginOverlap`
  (params (OtherActor :type "Actor Object Reference"))
  (if (`self.ActorHasTag` OtherActor "Candle")
    (`self.K2_DestroyActor` OtherActor)))

(fn `ChangeVisibilityGhostCamera`
  (params (ComponentToBeChanged :type "SceneComponent Object Reference"))
  (if (`KismetArrayLibrary.Array_IsNotEmpty` (`self.GetComponentsByTag` (`GameplayStatics.GetPlayerCharacter` 0) "/Script/Engine.CameraComponent" "GhostCamera"))
    (`SceneComponent.SetVisibility` ComponentToBeChanged true false)
    (else
      (`SceneComponent.SetVisibility` ComponentToBeChanged false false))))

(fn `UserConstructionScript`)