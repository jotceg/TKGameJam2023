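; Test pentagram prop with five BP_Candle child actor components, all hidden at BeginPlay.
; When an actor tagged "Ghost" overlaps it, the candle component nearest that actor is revealed if hidden.
; Tick checks whether all five candles report IsLight, with a "PENTAGRAM" debug print as the only result.
; A GhostCamera-based visibility helper is defined but not called here, and destroying the overlapping actor is left disconnected.
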(event `self.ReceiveBeginPlay`
  (`self.DisableCandels`))

(event `self.ReceiveActorBeginOverlap`
  (params (OtherActor :type "Actor Object Reference"))
  (if (`self.ActorHasTag` OtherActor "Ghost")
    (bind _newparam (`self.Find Closest Candle` (`SceneComponent.K2_GetComponentLocation` (`Actor.RootComponent` OtherActor))))
    (if (not (`SceneComponent.IsVisible` _newparam))
      (`SceneComponent.ToggleVisibility` _newparam false))))

(event `self.ReceiveTick`
  (params (DeltaSeconds :type "Float (single-precision)"))
  (bind _returnvalue (`self.AreLightsOn`))
  (`KismetSystemLibrary.PrintString` "PENTAGRAM" _returnvalue))

(fn `AreLightsOn`
  (returns (ReturnValue :type Boolean))
  (bind _asbp_candle (cast `/Game/MedievalDungeon/Blueprints/BP_Candle` (`ChildActorComponent.ChildActor` (`self.BP_Candle`)))
    (:`then`
      (bind _asbp_candle_2 (cast `/Game/MedievalDungeon/Blueprints/BP_Candle` (`ChildActorComponent.ChildActor` (`self.BP_Candle1`))))
      (bind _asbp_candle_3 (cast `/Game/MedievalDungeon/Blueprints/BP_Candle` (`ChildActorComponent.ChildActor` (`self.BP_Candle2`))))
      (bind _asbp_candle_4 (cast `/Game/MedievalDungeon/Blueprints/BP_Candle` (`ChildActorComponent.ChildActor` (`self.BP_Candle3`))))
      (bind _asbp_candle_5 (cast `/Game/MedievalDungeon/Blueprints/BP_Candle` (`ChildActorComponent.ChildActor` (`self.BP_Candle4`)))))
    (:`CastFailed`
      _))
  (return (and (and (and (`/Game/MedievalDungeon/Blueprints/BP_Candle.IsLight` _asbp_candle) (`/Game/MedievalDungeon/Blueprints/BP_Candle.IsLight` _asbp_candle_2)) (and (`/Game/MedievalDungeon/Blueprints/BP_Candle.IsLight` _asbp_candle_3) (`/Game/MedievalDungeon/Blueprints/BP_Candle.IsLight` _asbp_candle_4))) (`/Game/MedievalDungeon/Blueprints/BP_Candle.IsLight` _asbp_candle_5))))

(fn `ChangeVisibilityGhostCamera`
  (params (ComponentToBeChanged :type "SceneComponent Object Reference"))
  (if (`KismetArrayLibrary.Array_IsNotEmpty` (`self.GetComponentsByTag` (`GameplayStatics.GetPlayerCharacter` 0) "/Script/Engine.CameraComponent" "GhostCamera"))
    (`SceneComponent.SetVisibility` ComponentToBeChanged true false)
    (else
      (`SceneComponent.SetVisibility` ComponentToBeChanged false false))))

(fn `DisableCandels`
  (`SceneComponent.SetVisibility` (`self.BP_Candle`) false false)
  (`SceneComponent.SetVisibility` (`self.BP_Candle1`) false false)
  (`SceneComponent.SetVisibility` (`self.BP_Candle2`) false false)
  (`SceneComponent.SetVisibility` (`self.BP_Candle3`) false false)
  (`SceneComponent.SetVisibility` (`self.BP_Candle4`) false false))

(fn `Find Closest Candle`
  (params (`Overlaping Actor Location` :type "Vector Structure"))
  (returns (NewParam :type "ChildActorComponent Object Reference"))
  (bind _bp_candle (`self.BP_Candle`))
  (bind _bp_candle1 (`self.BP_Candle1`))
  (bind _bp_candle2 (`self.BP_Candle2`))
  (bind _bp_candle3 (`self.BP_Candle3`))
  (bind _bp_candle4 (`self.BP_Candle4`))
  (return (`|GetArrayItem` (`|MakeArray` _bp_candle _bp_candle1 _bp_candle2 _bp_candle3 _bp_candle4) (`KismetMathLibrary.MinOfFloatArray` (`|MakeArray` (`KismetMathLibrary.Vector_Distance` (`SceneComponent.K2_GetComponentLocation` _bp_candle) `Overlaping Actor Location`) (`KismetMathLibrary.Vector_Distance` (`SceneComponent.K2_GetComponentLocation` _bp_candle1) `Overlaping Actor Location`) (`KismetMathLibrary.Vector_Distance` (`SceneComponent.K2_GetComponentLocation` _bp_candle2) `Overlaping Actor Location`) (`KismetMathLibrary.Vector_Distance` (`SceneComponent.K2_GetComponentLocation` _bp_candle3) `Overlaping Actor Location`) (`KismetMathLibrary.Vector_Distance` (`SceneComponent.K2_GetComponentLocation` _bp_candle4) `Overlaping Actor Location`) :!type "Float (single-precision)")))))

(fn `UserConstructionScript`)