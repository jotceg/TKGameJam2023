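; Potion actor whose GhostSmoke component shows only while the player character has a camera component tagged GhostCamera.
; Tick queries player 0's character for that tagged camera every frame and sets the smoke's visibility from the result, without propagating to children.
; ChangeVisibilityGhostCamera repeats the same check for any component passed in, but nothing in this Blueprint calls it.
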(event `self.ReceiveTick`
  (params (DeltaSeconds :type "Float (single-precision)"))
  (bind _ghostsmoke (`self.GhostSmoke`))
  (if (`KismetArrayLibrary.Array_IsNotEmpty` (`self.GetComponentsByTag` (`GameplayStatics.GetPlayerCharacter` 0) "/Script/Engine.CameraComponent" "GhostCamera"))
    (`SceneComponent.SetVisibility` _ghostsmoke true false)
    (else
      (`SceneComponent.SetVisibility` _ghostsmoke false false))))

(fn `ChangeVisibilityGhostCamera`
  (params (ComponentToBeChanged :type "SceneComponent Object Reference"))
  (if (`KismetArrayLibrary.Array_IsNotEmpty` (`self.GetComponentsByTag` (`GameplayStatics.GetPlayerCharacter` 0) "/Script/Engine.CameraComponent" "GhostCamera"))
    (`SceneComponent.SetVisibility` ComponentToBeChanged true false)
    (else
      (`SceneComponent.SetVisibility` ComponentToBeChanged false false))))

(fn `UserConstructionScript`)